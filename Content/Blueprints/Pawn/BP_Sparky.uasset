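; Sparky player character: a Niagara particle body and trail that shrink with HP, with freeze jitter and a death timeline before the lose screen.
; Overlap tags pick the target of one input, which either zaps an enemy (damage plus stun) or interacts.
; Winning scores through the GameMode and turns XP into skill points for energy, agility and zap stats, persisted in the PlayerStats save.
; Also owns the UI widgets and C/G debug keys.
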(event `self.ReceiveBeginPlay`
  (`parent.ReceiveBeginPlay`)
  (bind _returnvalue (`GameplayStatics.DoesSaveGameExist` "PlayerStats"))
  (if _returnvalue
    (`self.Load Player Stats`)
    (else
      (`self.Create New Player Stats Save Game`)))
  (`self.Calculate Updated Player Stats`)
  (bind _returnvalue_2 (`|CreateWidget` "/Game/Blueprints/UMG/WB_UI_HUD.WB_UI_HUD_C"))
  (bind _output_get (set `self.UI_HUD` _returnvalue_2))
  (`UserWidget.AddToViewport` _output_get 0)
  (bind _returnvalue_3 (`|CreateWidget` "/Game/Blueprints/UMG/WB_LoseScreen.WB_LoseScreen_C"))
  (set `self.LoseScreen` _returnvalue_3)
  (bind _returnvalue_4 (`|CreateWidget` "/Game/Blueprints/UMG/WB_WinScreen.WB_WinScreen_C"))
  (set `self.WinScreen` _returnvalue_4)
  (bind _returnvalue_5 (`|CreateWidget` "/Game/Blueprints/UMG/WB_LvlUp.WB_LvlUp_C"))
  (set `self.Lvl Up UI ` _returnvalue_5)
  (`self.Update Particles Parameters By Health Amount`)
  (`GameplayStatics.PlaySound2D` (`self.Start Level Sound`) 1.0 1.0 0.0 "/Game/Assets/Audio/SCC_PlayerDamage.SCC_PlayerDamage" null)
  (message `/Game/Blueprints/Interface/BI_Timer.Start Timer` (`self.UI_HUD`))
  (`self.Check Evolve Status And Enable or Disable HUD Evolve Button`))

(event `self.ReceiveAnyDamage`
  (params (Damage :type "Float (single-precision)") (DamageType :type "DamageType Object Reference") (InstigatedBy :type "Controller Object Reference") (DamageCauser :type "Actor Object Reference"))
  (`self.IsAlive`
    (:`then`
      (message `/Game/Blueprints/Interface/BI_UMG_Calls.Play Hurt Screen Animation` (`self.UI_HUD`))
      (`GameplayStatics.PlaySound2D` (`self.Player Damage Sound`) 1.0 1.0 0.0 "/Game/Assets/Audio/SCC_PlayerDamage.SCC_PlayerDamage" null)
      (`self.Apply Damage To Self` Damage)
      (`self.Update Particles Parameters By Health Amount`))
    (:`else`
      (`/Game/Blueprints/Interface/BI_StopDamage.Stop Damage`))))

(event `/Game/Blueprints/Interface/BI_StopDamage.Stop Damage`
  (message `/Game/Blueprints/Interface/BI_UMG_Calls.Stop Hurt Screen Animation` (`self.UI_HUD`)))

(event `/Game/Blueprints/Interface/BI_PlayerProgress.HealPlayer`
  (params (`Heal Amount` :type "Float (double-precision)"))
  (`self.Heal Player` `Heal Amount`)
  (`self.Update Particles Parameters By Health Amount`))

(event `/Game/Blueprints/Interface/BI_PlayerProgress.AddScore`
  (params (`Score Points` :type Integer) (XP :type "Float (double-precision)"))
  (`self.Increase Score` `Score Points`)
  (`self.Increase XP` XP))

(event `Kill Player`
  (bind _charactermovement (`self.CharacterMovement`))
  (set `self.IsAlive` false)
  (`MovementComponent.StopMovementImmediately` _charactermovement)
  (`CharacterMovementComponent.DisableMovement` _charactermovement)
  (bind (_direction _particles_to_spawn) (`Timeline|Death Timeline`)
    (:`Update`
      (`FXSystemComponent.SetFloatParameter` (`self.Niagara`) "SpawnRate" _particles_to_spawn))
    (:`Finished`
      (`/Engine/EditorBlueprintResources/StandardMacros.DoOnce` false
        (:`Completed`
          (`ActorComponent.Deactivate` (`self.Niagara`))
          (`ActorComponent.Deactivate` (`self.Trail`))
          (`GameplayStatics.PlaySound2D` "/Game/Assets/Interface_And_Item_Sounds/Cues/Gong_01_Cue.Gong_01_Cue" 1.0 1.0 0.0 null null)
          (`self.Stop Timer And Get Time Result`)
          (`KismetSystemLibrary.Delay` 0.2)
          (`self.Show Lose Screen`))))))

(event `Key|C`
  (params (Key :type "Key Structure"))
  (:`Pressed`
    (`/Game/Blueprints/Interface/BI_PlayerProgress.AddScore` 0 200.0)))

(event `Key|G`
  (params (Key :type "Key Structure"))
  (:`Pressed`
    (`/Game/Blueprints/Interface/BI_EndLevel.Win Game`)))

(event `/Game/Blueprints/Interface/BI_EndLevel.Win Game`
  (`CharacterMovementComponent.DisableMovement` (`self.CharacterMovement`))
  (bind _achieved_time (`self.Stop Timer And Get Time Result`))
  (`self.Calculate Scores` _achieved_time)
  (`self.Increase Player Level`)
  (if (> (`self.Skill Points`) 0)
    (`self.Enable Win Screen Evolve Button`)
    (else
      (`self.Disable Win Screen Evolve Button`)))
  (`KismetSystemLibrary.Delay` 0.5)
  (`GameplayStatics.PlaySound2D` (`self.Win Level Audio`) 1.0 1.0 0.0 "/Game/Assets/Audio/SCC_PlayerDamage.SCC_PlayerDamage" null)
  (`self.Save All Player Stats`)
  (`self.Show Win Screen`))

(event `/Game/Blueprints/Interface/BI_EndLevel.Lose Game`
  (`self.Kill Player`))

(event `/Game/Blueprints/Interface/BI_EndLevel.Teleport Player`
  (params (Location :type "Vector Structure"))
  (`SceneComponent.K2_SetWorldLocation` (`self.CapsuleComponent`) Location false false))

(event `self.CapsuleComponent.OnComponentBeginOverlap`
  (params (OverlappedComponent :type "PrimitiveComponent Object Reference") (OtherActor :type "Actor Object Reference") (OtherComp :type "PrimitiveComponent Object Reference") (OtherBodyIndex :type Integer) (bFromSweep :type Boolean) (SweepResult :type "HitResult Structure (by ref)"))
  (for _array_element (`Actor.Tags` OtherActor)
    (switch `string` (`KismetStringLibrary.Conv_NameToString` _array_element)
      (:`Interact`
        (set `self.Interactable Actor` OtherActor))
      (:`Enemy`
        (set `self.Enemy Actor` OtherActor)))))

(event `self.CapsuleComponent.OnComponentEndOverlap`
  (params (OverlappedComponent :type "PrimitiveComponent Object Reference") (OtherActor :type "Actor Object Reference") (OtherComp :type "PrimitiveComponent Object Reference") (OtherBodyIndex :type Integer))
  (for _array_element (`Actor.Tags` OtherActor)
    (switch `string` (`KismetStringLibrary.Conv_NameToString` _array_element)
      (:`Interact`
        (set `self.Interactable Actor` null))
      (:`Enemy`
        (set `self.Enemy Actor` null)))))

(event `EnhancedInput|/Game/Variant_SideScroller/Input/Actions/IA_Interact`
  (params (ActionValue :type Boolean) (ElapsedSeconds :type "Float (double-precision)") (TriggeredSeconds :type "Float (double-precision)") (InputAction :type "InputAction Object Reference" :default "/Game/Variant_SideScroller/Input/Actions/IA_Interact.IA_Interact"))
  (:`Started`
    (`/Engine/EditorBlueprintResources/StandardMacros.DoOnce` false :!label _label
      (:`Completed`
        (`self.Zap or Interact`))))
  (:`Completed`
    (goto _label :!via `Reset`)))

(event `/Game/Blueprints/Interface/BI_StopAllMovement.Freeze`
  (params (Duration :type "Float (double-precision)"))
  (`self.Freeze Player`)
  (`KismetSystemLibrary.Delay` Duration)
  (`/Game/Blueprints/Interface/BI_StopAllMovement.Unfreeze`))

(event `/Game/Blueprints/Interface/BI_StopAllMovement.Unfreeze`
  (`self.Stop Jitter and Reactivate Movement`))

(event `/Game/Blueprints/Interface/BI_UMG_Calls.Zap or Interact`
  (`self.Activate Zap Effects`)
  (`self.Interact or Zap Enemy`))

(event `/Game/Blueprints/Interface/BI_UMG_Calls.Save Skill Lvls`
  (params (`Energy Lvl` :type Integer) (`Agility Lvl` :type Integer) (`Zap Lvl` :type Integer) (`Skill Points` :type Integer))
  (`self.Update Leveled Stats` `Energy Lvl` `Agility Lvl` `Zap Lvl` `Skill Points`)
  (`self.Save Level Up Stats`)
  (`self.Calculate Updated Player Stats`)
  (`self.Save All Player Stats`))

(event `/Game/Blueprints/Interface/BI_UMG_Calls.Open Lvl Up UI`
  (bind _lvl_up_ui_ (`self.Lvl Up UI `))
  (if (`Widget.IsInViewport` (`self.WinScreen`))
    (`UserWidget.AddToViewport` (`self.Lvl Up UI `) 0)
    (else
      (message `/Game/Blueprints/Interface/BI_Timer.Stop Timer` (`/Game/Blueprints/UMG/WB_UI_HUD.WB_Timer` (`self.UI_HUD`)))
      (`GameplayStatics.SetGamePaused` true)
      (`UserWidget.AddToViewport` _lvl_up_ui_ 0)
      (`WidgetBlueprintLibrary.SetInputMode_UIOnlyEx` (`GameplayStatics.GetPlayerController` 0) _lvl_up_ui_))))

(event `/Game/Blueprints/Interface/BI_UMG_Calls.Close Lvl Up UI`
  (if (`Widget.IsInViewport` (`self.WinScreen`))
    (`Widget.RemoveFromParent` (`self.Lvl Up UI `))
    (`self.Check Evolve Status And Enable or Disable HUD Evolve Button`)
    (`self.Check Skill Points and Enable or Disable Win Screen Evolve Button`)
    (else
      (`Widget.RemoveFromParent` (`self.Lvl Up UI `))
      (`WidgetBlueprintLibrary.SetInputMode_GameAndUIEx` (`GameplayStatics.GetPlayerController` 0) (`self.UI_HUD`))
      (`GameplayStatics.SetGamePaused` false)
      (message `/Game/Blueprints/Interface/BI_Timer.Start Timer` (`self.UI_HUD`))
      (`self.Check Evolve Status And Enable or Disable HUD Evolve Button`))))

(fn `Activate Zap Effects`
  (bind _ns_zap (`self.NS_Zap`))
  (if (`ActorComponent.IsActive` _ns_zap)
    (`ActorComponent.Deactivate` _ns_zap))
  (`ActorComponent.Activate` _ns_zap false)
  (`GameplayStatics.PlaySound2D` (`self.Zap Sound`) 1.0 1.0 0.0 null null))

(fn `Apply Damage To Self`
  (params (Damage :type "Float (double-precision)"))
  (bind _output_get (set `self.HP` (`KismetMathLibrary.FClamp` (- (`self.HP`) Damage) 0.0 (`self.MaxHP`))))
  (if (== _output_get 0.0)
    (`self.Kill Player`)))

(fn `Calculate Scores`
  (params (Time :type "Float (double-precision)"))
  (bind _returnvalue (`GameplayStatics.GetGameMode`))
  (message `/Game/Blueprints/Interface/BI_GetData.CompleteLevelScore` _returnvalue (`self.Score`) Time)
  (bind (_final_score _high_score) (message `/Game/Blueprints/Interface/BI_GetData.CalculateFinalScore` _returnvalue))
  (set `self.Score` _final_score)
  (set `self.High Score` _high_score))

(fn `Calculate Updated Player Stats`
  (set `self.Player Speed` (+ (`self.Base Speed`) (* (`self.Agility LVL`) (`self.Speed Per Level Multiplier`))))
  (bind _output_get (set `self.MaxHP` (+ (`self.Base HP`) (* (`self.Energy LVL`) (`self.HP Per Level Multiplier`)))))
  (set `self.HP` _output_get)
  (set `self.Zap Stun Duration` (+ (`self.Base Stun Duration`) (* (`self.Zap LVL`) (`self.Stun Duration Per Level Multiplier`))))
  (set `self.Zap Dmg` (+ (`self.Base Zap Damage`) (* (`self.Zap LVL`) (`self.Zap Dmg Per Level Multiplier`))))
  (`self.Update Player Speed`))

(fn `CalculateFinalScore`
  (returns (`Final Score` :type Integer) (`High Score` :type Integer) (`Collected Pickups` :type Integer) (`Max Collectibles` :type Integer) (`Completion Time` :type Integer))
  (return 0 0 0 0 0))

(fn `Check Evolve Status And Enable or Disable HUD Evolve Button`
  (bind _button_evolve (`/Game/Blueprints/UMG/WB_UI_HUD.Button_Evolve` (`self.UI_HUD`)))
  (if (> (`self.Skill Points`) 0)
    (`Widget.SetIsEnabled` _button_evolve true)
    (`Widget.SetVisibility` _button_evolve "Visible")
    (else
      (`Widget.SetIsEnabled` _button_evolve false)
      (`Widget.SetVisibility` _button_evolve "Hidden"))))

(fn `Check Skill Points and Enable or Disable Win Screen Evolve Button`
  (if (> (`self.Skill Points`) 0)
    (`self.Enable Win Screen Evolve Button`)
    (else
      (`self.Disable Win Screen Evolve Button`))))

(fn `Create New Player Stats Save Game`
  (bind _returnvalue (`GameplayStatics.CreateSaveGameObject` "/Game/Saves/SavePlayerProgress.SavePlayerProgress_C"))
  (set `self.Save Stats Ref` _returnvalue)
  (message `/Game/Blueprints/Interface/BI_SaveHandler.SaveStats` (`self.Save Stats Ref`) (`self.HP`) (`self.MaxHP`) (`self.XP`) (`self.LVL`) (`self.Zap LVL`) (`self.Zap Dmg`) (`self.Zap Stun Duration`) (`self.Energy LVL`) (`self.Agility LVL`) (`self.Player Speed`) (`self.Skill Points`) (`self.Lvl XP`))
  (`GameplayStatics.SaveGameToSlot` (`self.Save Stats Ref`) "PlayerStats"))

(fn `Disable Win Screen Evolve Button`
  (bind _button_evolve (`/Game/Blueprints/UMG/WB_WinScreen.Button_Evolve` (`self.WinScreen`)))
  (`Widget.SetIsEnabled` _button_evolve false)
  (`Widget.SetVisibility` _button_evolve "Hidden"))

(fn `Enable Win Screen Evolve Button`
  (bind _button_evolve (`/Game/Blueprints/UMG/WB_WinScreen.Button_Evolve` (`self.WinScreen`)))
  (`Widget.SetIsEnabled` _button_evolve true)
  (`Widget.SetVisibility` _button_evolve "Visible"))

(fn `Freeze Player`
  (`MovementComponent.StopMovementImmediately` (`self.CharacterMovement`))
  (`CharacterMovementComponent.DisableMovement` (`self.CharacterMovement`))
  (`FXSystemComponent.SetFloatParameter` (`self.Niagara`) "Jitter Amount" (`self.Jitter Amount`)))

(fn `Get Skill Points And Skill Lvls`
  (returns (`Skill Points` :type Integer) (`Energy Lvl` :type Integer) (`Agility Lvl` :type Integer) (`Zap Lvl` :type Integer))
  (return (`self.Skill Points`) (`self.Energy LVL`) (`self.Agility LVL`) (`self.Zap LVL`)))

(fn `GetAllScores`
  (returns (`Final Score` :type Integer) (`High Score` :type Integer) (`Collected Pickups` :type Integer) (`Max Collectibles` :type Integer) (`Completion Time` :type "Float (double-precision)") (`Enemies Spawned` :type Integer) (`Enemies Defeated` :type Integer) (`Current Player Score` :type Integer) (`Minus Score Per Second` :type Integer) (`Level Completion Time Int` :type Integer) (`Minus Timer Score` :type Integer))
  (return 0 0 0 0 0.0 0 0 0 0 0 0))

(fn `GetLastPlayedLevel`
  (returns (LastPlayedLevel :type Name))
  (return "None"))

(fn `GetScore`
  (returns (Score :type Integer))
  (return (`self.Score`)))

(fn `Heal Player`
  (params (A :type "Float (double-precision)"))
  (set `self.HP` (`KismetMathLibrary.FClamp` (+ A (`self.HP`)) 0.0 (`self.MaxHP`))))

(fn `Increase Player Level`
  (if (>= (`self.XP`) (`self.Lvl XP`)) :!label _label
    (if (!= (`self.LVL`) (`self.Max LVL`))
      (set `self.XP` (- (`self.XP`) (`self.Lvl XP`)))
      (`/Engine/EditorBlueprintResources/StandardMacros.IncrementInt` (`self.LVL`)
        (:`  `
          (`/Engine/EditorBlueprintResources/StandardMacros.IncrementInt` (`self.Skill Points`)
            (:`  `
              (bind _output_get (set `self.Lvl XP` (+ (`self.Lvl XP`) (* (`self.LVL`) (`self.XP per Lvl Up`)))))
              (if (>= (`self.XP`) _output_get)
                (goto _label)))))))
    (elif (== (`self.LVL`) (`self.Max LVL`))
      (set `self.isMaxLvl` true))))

(fn `Increase Score`
  (params (B :type Integer))
  (set `self.Score` (+ (`self.Score`) B)))

(fn `Increase XP`
  (params (XP :type "Float (double-precision)"))
  (`self.isMaxLvl`
    (:`then`
      (set `self.XP` (`self.Lvl XP`)))
    (:`else`
      (set `self.XP` (+ (`self.XP`) XP)))))

(fn `Interact or Zap Enemy`
  (switch `int` (`KismetMathLibrary.SelectInt` 1 0 (`KismetSystemLibrary.IsValid` (`self.Enemy Actor`)))
    (:`0`
      (message `/Game/Blueprints/Interface/BI_Interact.Interact` (`self.Interactable Actor`)))
    (:`1`
      (`GameplayStatics.ApplyDamage` (`self.Enemy Actor`) (`self.Zap Dmg`))
      (message `/Game/Blueprints/Interface/BI_StopAllMovement.Freeze` (`self.Enemy Actor`) (`self.Zap Stun Duration`)))))

(fn `Load Player Stats`
  (bind _returnvalue (`GameplayStatics.LoadGameFromSlot` "PlayerStats"))
  (bind _assave_player_progress (cast `/Game/Saves/SavePlayerProgress` _returnvalue))
  (bind _output_get (set `self.Save Stats Ref` _assave_player_progress))
  (bind (_hp _max_hp _xp _lvl _zap_lvl _zap_dmg _zap_stun_duration _energy_lvl _agility_lvl _player_speed _skill_points _lvl_xp) (message `/Game/Blueprints/Interface/BI_SaveHandler.LoadStats` _output_get))
  (set `self.HP` _hp)
  (set `self.MaxHP` _max_hp)
  (set `self.XP` _xp)
  (set `self.LVL` _lvl)
  (set `self.Zap LVL` _zap_lvl)
  (set `self.Zap Dmg` _zap_dmg)
  (set `self.Zap Stun Duration` _zap_stun_duration)
  (set `self.Energy LVL` _energy_lvl)
  (set `self.Agility LVL` _agility_lvl)
  (set `self.Player Speed` _player_speed)
  (set `self.Skill Points` _skill_points)
  (set `self.Lvl XP` _lvl_xp))

(fn `Save All Player Stats`
  (bind _returnvalue (`GameplayStatics.DoesSaveGameExist` "PlayerStats"))
  (if _returnvalue
    (if (`KismetSystemLibrary.DoesImplementInterface` (`self.Save Stats Ref`) "/Game/Blueprints/Interface/BI_SaveHandler.BI_SaveHandler_C")
      (message `/Game/Blueprints/Interface/BI_SaveHandler.SaveStats` (`self.Save Stats Ref`) (`self.HP`) (`self.MaxHP`) (`self.XP`) (`self.LVL`) (`self.Zap LVL`) (`self.Zap Dmg`) (`self.Zap Stun Duration`) (`self.Energy LVL`) (`self.Agility LVL`) (`self.Player Speed`) (`self.Skill Points`) (`self.Lvl XP`))
      (`GameplayStatics.SaveGameToSlot` (`self.Save Stats Ref`) "PlayerStats")
      (else
        (`KismetSystemLibrary.PrintString` "SAVE GAME REF DOES NOT IMPLEMENT INTERFACE" true true (struct :`R` 1.0 :`G` 0.018587 :`B` 0.015625 :`A` 1.0) 5.0)))))

(fn `Save Level Up Stats`
  (bind _save_stats_ref (`self.Save Stats Ref`))
  (set `/Game/Saves/SavePlayerProgress.Skill Points` (`self.Skill Points`) _save_stats_ref)
  (set `/Game/Saves/SavePlayerProgress.Energy LVL` (`self.Energy LVL`) _save_stats_ref)
  (set `/Game/Saves/SavePlayerProgress.Agility LVL` (`self.Agility LVL`) _save_stats_ref)
  (set `/Game/Saves/SavePlayerProgress.Zap LVL` (`self.Zap LVL`) _save_stats_ref)
  (`GameplayStatics.SaveGameToSlot` (`self.Save Stats Ref`) "PlayerStats"))

(fn `SendUIStats`
  (returns (HP :type "Float (double-precision)") (MaxHP :type "Float (double-precision)") (LVL :type Integer) (XP :type "Float (double-precision)") (LevelXP :type "Float (double-precision)"))
  (return (`self.HP`) (`self.MaxHP`) (`self.LVL`) (`self.XP`) (`self.Lvl XP`)))

(fn `Show Lose Screen`
  (bind _returnvalue (`GameplayStatics.GetPlayerController` 0))
  (`UserWidget.AddToViewport` (`self.LoseScreen`) 0)
  (set `PlayerController.bShowMouseCursor` true _returnvalue)
  (`WidgetBlueprintLibrary.SetInputMode_UIOnlyEx` _returnvalue (`self.LoseScreen`)))

(fn `Show Win Screen`
  (bind _returnvalue (`GameplayStatics.GetPlayerController` 0))
  (bind _winscreen (`self.WinScreen`))
  (`UserWidget.AddToViewport` _winscreen 0)
  (`GameplayStatics.SetGamePaused` true)
  (set `PlayerController.bShowMouseCursor` true _returnvalue)
  (`WidgetBlueprintLibrary.SetInputMode_UIOnlyEx` _returnvalue _winscreen))

(fn `Stop Jitter and Reactivate Movement`
  (`CharacterMovementComponent.SetMovementMode` (`self.CharacterMovement`) "MOVE_Walking" 0)
  (`FXSystemComponent.SetFloatParameter` (`self.Niagara`) "Jitter Amount" 0.0))

(fn `Stop Timer And Get Time Result`
  (returns (`Achieved Time` :type "Float (double-precision)"))
  (bind _achieved_time (message `/Game/Blueprints/Interface/BI_Timer.Stop Timer` (`/Game/Blueprints/UMG/WB_UI_HUD.WB_Timer` (`self.UI_HUD`))))
  (return _achieved_time))

(fn `Update Leveled Stats`
  (params (`Energy LVL` :type Integer) (`Agility LVL` :type Integer) (`Zap LVL` :type Integer) (`Skill Points` :type Integer))
  (set `self.Energy LVL` `Energy LVL`)
  (set `self.Agility LVL` `Agility LVL`)
  (set `self.Zap LVL` `Zap LVL`)
  (set `self.Skill Points` `Skill Points`))

(fn `Update Particles Parameters By Health Amount`
  (bind _niagara (`self.Niagara`))
  (bind _trail (`self.Trail`))
  (`NiagaraComponent.SetVariableFloat` _niagara "Sprite Size" (* (`self.Max Sprite Size`) (/ (`self.HP`) (`self.MaxHP`))))
  (`FXSystemComponent.SetFloatParameter` _niagara "Lifetime Min" (* (`self.Min Lifetime `) (/ (`self.HP`) (`self.MaxHP`))))
  (`FXSystemComponent.SetFloatParameter` _niagara "Lifetime Max" (* (`self.Max Lifetime`) (/ (`self.HP`) (`self.MaxHP`))))
  (`FXSystemComponent.SetFloatParameter` (`self.Niagara`) "Sphere Radius" (* (`self.Max Sphere Radius`) (/ (`self.HP`) (`self.MaxHP`))))
  (`FXSystemComponent.SetFloatParameter` _trail "Scale Curve_Ribbon Width" (* (`self.Max Ribbon Size`) (/ (`self.HP`) (`self.MaxHP`))))
  (`FXSystemComponent.SetFloatParameter` _trail "Sphere Radius" (* (`self.Max Ribbon Sphere Radius`) (/ (`self.HP`) (`self.MaxHP`)))))

(fn `Update Player Speed`
  (set `CharacterMovementComponent.MaxWalkSpeed` (`self.Player Speed`) (`self.CharacterMovement`)))

(fn `UserConstructionScript`)