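; BP_MovingWall is a wall moved by an InterpToMovement component that can be switched on and off through interaction.
; BeginPlay sets the component's tick from the IsEnabled state.
; Interact calls Open, which toggles both that tick and IsEnabled, so movement pauses or runs.
; GetActiveStatus always returns false, regardless of that state.
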(event `self.ReceiveBeginPlay`
  (`self.IsEnabled`
    (:`then`
      (`ActorComponent.SetComponentTickEnabled` (`self.InterpToMovement`) true))
    (:`else`
      (`ActorComponent.SetComponentTickEnabled` (`self.InterpToMovement`) false))))

(event `/Game/Blueprints/Interface/BI_Interact.Open`
  (`self.IsEnabled`
    (:`then`
      (`ActorComponent.SetComponentTickEnabled` (`self.InterpToMovement`) false)
      (set `self.IsEnabled` false))
    (:`else`
      (`ActorComponent.SetComponentTickEnabled` (`self.InterpToMovement`) true)
      (set `self.IsEnabled` true))))

(event `/Game/Blueprints/Interface/BI_Interact.Interact`
  (`/Game/Blueprints/Interface/BI_Interact.Open`))

(fn `GetActiveStatus`
  (returns (isActivated :type Boolean))
  (return false))

(fn `UserConstructionScript`)