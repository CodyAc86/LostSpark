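; BP_Finish_Pad is a finish pad that triggers the win when the player reaches it.
; When the player character overlaps the Capsule, it sends that character a teleport message with the capsule's location, activates the Niagara effect, then sends the win-game message.
; Hide and ShowHidden events toggle the pad's visibility and collision together.
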(event `self.Capsule.OnComponentBeginOverlap`
  (params (OverlappedComponent :type "PrimitiveComponent Object Reference") (OtherActor :type "Actor Object Reference") (OtherComp :type "PrimitiveComponent Object Reference") (OtherBodyIndex :type Integer) (bFromSweep :type Boolean) (SweepResult :type "HitResult Structure (by ref)"))
  (bind _returnvalue (`GameplayStatics.GetPlayerCharacter` 0))
  (if (== OtherActor _returnvalue)
    (message `/Game/Blueprints/Interface/BI_EndLevel.Teleport Player` _returnvalue (`SceneComponent.K2_GetComponentLocation` (`self.Capsule`)))
    (`ActorComponent.Activate` (`self.Niagara`) false)
    (message `/Game/Blueprints/Interface/BI_EndLevel.Win Game` _returnvalue)))

(event `/Game/Blueprints/Interface/BI_HiddenHandler.Hide`
  (`self.SetActorHiddenInGame` true)
  (`self.SetActorEnableCollision` false))

(event `/Game/Blueprints/Interface/BI_HiddenHandler.Show Hidden`
  (`self.SetActorHiddenInGame` false)
  (`self.SetActorEnableCollision` true))

(fn `UserConstructionScript`)