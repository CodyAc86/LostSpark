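; Moving platform, remote no-loop variant, that the player switches on and off by interacting with its energy core.
; A box overlap with the player pawn highlights the core via overlay material and allows interaction.
; Interact fires a Niagara effect, swaps the core's emissive material, and toggles InterpToMovement ticking and root mobility between Static and Movable.
; BeginPlay applies the initial IsEnabled state to movement ticking only; GetActiveStatus always returns false.
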(event `self.ReceiveBeginPlay`
  (`self.IsEnabled`
    (:`then`
      (`ActorComponent.SetComponentTickEnabled` (`self.InterpToMovement`) true))
    (:`else`
      (`ActorComponent.SetComponentTickEnabled` (`self.InterpToMovement`) false))))

(event `self.Box.OnComponentBeginOverlap`
  (params (OverlappedComponent :type "PrimitiveComponent Object Reference") (OtherActor :type "Actor Object Reference") (OtherComp :type "PrimitiveComponent Object Reference") (OtherBodyIndex :type Integer) (bFromSweep :type Boolean) (SweepResult :type "HitResult Structure (by ref)"))
  (if (== OtherActor (`GameplayStatics.GetPlayerPawn` 0))
    (`MeshComponent.SetOverlayMaterial` (`self.SM_EnergyCore_A`) "/Game/Blueprints/Materials/MI_HighlightMat_Inst.MI_HighlightMat_Inst")
    (set `self.CanInteract` true)))

(event `self.Box.OnComponentEndOverlap`
  (params (OverlappedComponent :type "PrimitiveComponent Object Reference") (OtherActor :type "Actor Object Reference") (OtherComp :type "PrimitiveComponent Object Reference") (OtherBodyIndex :type Integer))
  (if (== OtherActor (`GameplayStatics.GetPlayerPawn` 0))
    (`MeshComponent.SetOverlayMaterial` (`self.SM_EnergyCore_A`) null)
    (set `self.CanInteract` false)))

(event `self.Interact`
  (`self.CanInteract`
    (:`then`
      (`ActorComponent.Activate` (`self.Niagara`) false)
      (`self.IsEnabled`
        (:`then`
          (`PrimitiveComponent.SetMaterialByName` (`self.SM_EnergyCore_A`) "EnergyEmissive_A" "/Game/StarterBundle/ModularScifiHallways/Materials/MI_EnergyEmissive_A.MI_EnergyEmissive_A")
          (`ActorComponent.SetComponentTickEnabled` (`self.InterpToMovement`) false)
          (`SceneComponent.SetMobility` (`self.DefaultSceneRoot`) "Static")
          (set `self.IsEnabled` false))
        (:`else`
          (`PrimitiveComponent.SetMaterialByName` (`self.SM_EnergyCore_A`) "EnergyEmissive_A" "/Game/StarterBundle/ModularScifiHallways/Materials/MI_EnergyEmissive_B.MI_EnergyEmissive_B")
          (`ActorComponent.SetComponentTickEnabled` (`self.InterpToMovement`) true)
          (`SceneComponent.SetMobility` (`self.DefaultSceneRoot`) "Movable")
          (set `self.IsEnabled` true))))
    (:`else`)))

(fn `GetActiveStatus`
  (returns (isActivated :type Boolean))
  (return false))

(fn `UserConstructionScript`)