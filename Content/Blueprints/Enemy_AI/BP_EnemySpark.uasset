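; BP_EnemySpark is an enemy that wanders until it detects the player, then chases and latches onto them.
; A LookForPlayer loop drives AI MoveTo and snap-attaches within attack range, while overlap starts a looping damage timer and enlarges its particles.
; Freeze detaches and immobilizes it with a particle tint until Unfreeze resumes the loop.
; At zero health it awards score and XP, notifies the game mode and destroys itself.
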(event `self.ReceiveBeginPlay`
  (`self.Look for Player`))

(event `self.ReceiveTick`
  (params (DeltaSeconds :type "Float (single-precision)"))
  (if (`self.Is In Detection Distance`)
    (`/Engine/EditorBlueprintResources/StandardMacros.DoOnce` false
      (:`Completed`
        (set `self.is Player Detected` true)))))

(event `self.ReceiveAnyDamage`
  (params (Damage :type "Float (single-precision)") (DamageType :type "DamageType Object Reference") (InstigatedBy :type "Controller Object Reference") (DamageCauser :type "Actor Object Reference"))
  (`self.Decrease Health` Damage))

(event `Kill AI`
  (`self.Add Score And Destroy Actor`))

(event `Look for Player`
  (`self.isStunned`
    (:`then`)
    (:`else`
      (`/Engine/EditorBlueprintResources/StandardMacros.IsValid` (`GameplayStatics.GetPlayerPawn` 0)
        (:`Is Valid`
          (`self.is Player Detected`
            (:`then`
              (if (`self.Is In Attack Distance`)
                (`self.K2_SetActorTransform` (`self.GetTransform` (`GameplayStatics.GetPlayerCharacter` 0)))
                (`self.K2_AttachToActor` (`self.Player Actor`) "None" "SnapToTarget" "SnapToTarget" "KeepRelative")
                (else
                  (`|AIMoveTo` self (0.0 0.0 0.0) (`GameplayStatics.GetPlayerCharacter` 0)
                    (:`OnSuccess`
                      (`self.Look for Player`))
                    (:`OnFail`
                      (`self.Look for Player`))))))
            (:`else`
              (`self.MoveToRandomLocation`))))))))

(event `MoveToRandomLocation`
  (`self.is Player Detected`
    (:`then`
      (`self.Look for Player`))
    (:`else`
      (`|AIMoveTo` self (`NavigationSystemV1.K2_GetRandomReachablePointInRadius` (`self.K2_GetActorLocation`) 50.0 null null) null
        (:`OnSuccess`
          _)
        (:`OnFail`
          _))
      (`self.Look for Player`))))

(event `self.ReceiveActorBeginOverlap`
  (params (OtherActor :type "Actor Object Reference"))
  (`/Engine/EditorBlueprintResources/StandardMacros.IsValid` OtherActor
    (:`Is Valid`
      (if (== OtherActor (`GameplayStatics.GetPlayerCharacter` 0))
        (set `self.Player Actor` OtherActor)
        (`NiagaraComponent.SetVariableFloat` (`self.Particles`) "Sphere Radius" 90.0)
        (`/Engine/EditorBlueprintResources/StandardMacros.IsValid` (`GameplayStatics.GetPlayerCharacter` 0)
          (:`Is Valid`
            (`KismetSystemLibrary.K2_SetTimerDelegate` (delegate `StartDamage`) 0.05 true)))))))

(event `StartDamage`
  (bind _returnvalue (`GameplayStatics.GetPlayerCharacter` 0))
  (`/Engine/EditorBlueprintResources/StandardMacros.IsValid` _returnvalue
    (:`Is Valid`
      (if (`PrimitiveComponent.IsOverlappingActor` (`self.CapsuleComponent`) _returnvalue)
        (`GameplayStatics.ApplyDamage` (`GameplayStatics.GetPlayerCharacter` 0) (`self.Base Damage`))
        (else
          (`self.K2_DetachFromActor` "KeepWorld" "KeepWorld" "KeepWorld")
          (`NiagaraComponent.SetVariableFloat` (`self.Particles`) "Sphere Radius" 30.0)
          (`/Engine/EditorBlueprintResources/StandardMacros.DoOnce` false :!label _label
            (:`Completed`
              (message `/Game/Blueprints/Interface/BI_StopDamage.Stop Damage` (`GameplayStatics.GetPlayerCharacter` 0))
              (`self.Look for Player`)
              (goto _label :!via `Reset`))))))))

(event `self.ReceiveActorEndOverlap`
  (params (OtherActor :type "Actor Object Reference"))
  (`self.Look for Player`))

(event `/Game/Blueprints/Interface/BI_StopAllMovement.Freeze`
  (params (Duration :type "Float (double-precision)"))
  (bind _charactermovement (`self.CharacterMovement`))
  (bind _particles (`self.Particles`))
  (set `self.Duration` Duration)
  (set `self.isStunned` true)
  (`self.K2_DetachFromActor` "KeepWorld" "KeepWorld" "KeepWorld")
  (`MovementComponent.StopMovementImmediately` _charactermovement)
  (`CharacterMovementComponent.DisableMovement` _charactermovement)
  (`FXSystemComponent.SetColorParameter` _particles "Color Maximum" (struct :`R` 0.20794 :`G` 0.245396 :`B` 1.0 :`A` 1.0))
  (`FXSystemComponent.SetFloatParameter` _particles "Sphere Radius" 70.0)
  (`KismetSystemLibrary.Delay` (`self.Duration`))
  (`/Game/Blueprints/Interface/BI_StopAllMovement.Unfreeze`))

(event `/Game/Blueprints/Interface/BI_StopAllMovement.Unfreeze`
  (bind _particles (`self.Particles`))
  (`FXSystemComponent.SetColorParameter` _particles "Color Maximum" (`self.Default Color Param`))
  (`FXSystemComponent.SetFloatParameter` _particles "Sphere Radius" (`self.Default Sphere Radius`))
  (`CharacterMovementComponent.SetMovementMode` (`self.CharacterMovement`) "MOVE_Walking" 0)
  (set `self.isStunned` false)
  (`self.Look for Player`))

(event `/Game/Blueprints/Interface/BI_EnemyAI.JumpToDestination`
  (params (Destination :type "Vector Structure"))
  (bind _outlaunchvelocity (`GameplayStatics.SuggestProjectileVelocity_CustomArc` (`self.K2_GetActorLocation`) (`KismetMathLibrary.MakeVector` (.x Destination) 1000.0 (+ (.z Destination) 100.0))))
  (`self.LaunchCharacter` _outlaunchvelocity true true)
  (`self.Look for Player`))

(fn `Add Score And Destroy Actor`
  (bind _returnvalue (`GameplayStatics.GetPlayerCharacter` 0))
  (message `/Game/Blueprints/Interface/BI_PlayerProgress.AddScore` _returnvalue (`self.Score Points`) (`self.XpPerKill`))
  (message `/Game/Variant_SideScroller/Blueprints/BPI_SideScrolling.Register Kill` (`GameplayStatics.GetGameMode`))
  (`GameplayStatics.PlaySound2D` (`self.Kill AI Sound`) 1.0 1.0 0.0 "/Game/Assets/Audio/SCC_PlayerDamage.SCC_PlayerDamage" null)
  (message `/Game/Blueprints/Interface/BI_StopDamage.Stop Damage` _returnvalue)
  (`self.K2_DestroyActor`))

(fn `Decrease Health`
  (params (`Damage Amount` :type "Float (double-precision)"))
  (bind _output_get (set `self.HP` (`KismetMathLibrary.FClamp` (- (`self.HP`) `Damage Amount`) 0.0 (`self.Max HP`))))
  (if (== _output_get 0.0)
    (set `self.Dead` true)
    (`self.Kill AI`)
    (else
      (return))))

(fn `Is In Attack Distance`
  (returns (ReturnValue :type Boolean))
  (return (<= (`self.GetDistanceTo` (`GameplayStatics.GetPlayerCharacter` 0)) (`self.Attack Distance`))))

(fn `Is In Detection Distance`
  (returns (ReturnValue :type Boolean))
  (return (<= (`self.GetDistanceTo` (`GameplayStatics.GetPlayerPawn` 0)) (`self.DetectionDistance`))))

(fn `UserConstructionScript`)