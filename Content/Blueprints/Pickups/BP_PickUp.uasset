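; Player-only pickup actor that heals the player and awards score and XP when collected.
; The first player overlap plays a sound, removes collision, then notifies the Game Mode and player through message calls.
; Two chained timelines animate Niagara sprite and cylinder sizes before the actor destroys itself.
; Hide and ShowHidden toggle visibility and collision, while key getters return only zeros.
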(event `self.ReceiveActorBeginOverlap`
  (params (OtherActor :type "Actor Object Reference"))
  (bind _returnvalue (`GameplayStatics.GetPlayerPawn` 0))
  (bind _ns_pickups (`self.NS_Pickups`))
  ; If the Player overlaps the collision sphere, inform the Game Mode that the pickup has been "collected" via an interface, heal the player and then delete self
  (if (== OtherActor (`GameplayStatics.GetPlayerPawn` 0))
    (`/Engine/EditorBlueprintResources/StandardMacros.DoOnce` false
      (:`Completed`
        (`GameplayStatics.PlaySound2D` "/Game/Assets/Interface_And_Item_Sounds/Cues/Special_Powerup_02_Cue.Special_Powerup_02_Cue" 1.0 1.0 0.0 null null)
        (`ActorComponent.K2_DestroyComponent` (`self.Collision`))
        (message `/Game/Variant_SideScroller/Blueprints/BPI_SideScrolling.Interaction` (`GameplayStatics.GetGameMode`) self)
        (message `/Game/Blueprints/Interface/BI_PlayerProgress.HealPlayer` _returnvalue (`self.HealAmount`))
        (message `/Game/Blueprints/Interface/BI_PlayerProgress.AddScore` _returnvalue (`self.Score Points`) (`self.XpPerPickup`))
        (bind (_direction _scalefloat) (`Timeline|PopOut` :!via `PlayFromStart`)
          (:`Update`
            (`NiagaraComponent.SetVariableFloat` _ns_pickups "Uniform Sprite Size" _scalefloat))
          (:`Finished`
            (bind (_direction_2 _scalecillinderfloat) (`Timeline|Timeline` :!via `PlayFromStart`)
              (:`Update`
                (`NiagaraComponent.SetVariableFloat` _ns_pickups "Cylinder Size" _scalecillinderfloat))
              (:`Finished`
                (`self.K2_DestroyActor`)))))))))

(event `/Game/Blueprints/Interface/BI_HiddenHandler.Hide`
  (`self.SetActorHiddenInGame` true)
  (`self.SetActorEnableCollision` false))

(event `/Game/Blueprints/Interface/BI_HiddenHandler.Show Hidden`
  (`self.SetActorHiddenInGame` false)
  (`self.SetActorEnableCollision` true))

(fn `Get Key Input`
  (returns (`Input 1` :type Integer) (`Input 2` :type Integer) (`Input 3` :type Integer))
  (return 0 0 0))

(fn `Get Pass Key`
  (returns (`Key 1` :type Integer) (`Key 2` :type Integer) (`Key 3` :type Integer))
  (return 0 0 0))

(fn `UserConstructionScript`)