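; One-shot trigger that reveals and hides tagged actors when the player pawn overlaps its box.
; On BeginPlay it gathers both groups by tag and sends hide messages to those awaiting reveal.
; On trigger it recolors its Niagara effect green, swaps both groups via messages, plays a sound if any are revealed, then destroys itself after a delay.
; Its own show/hide events toggle effect, visibility and collision.
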(event `self.ReceiveBeginPlay`
  (`self.Get Tagged Actors and Save in Array`)
  (for _array_element (`self.Hidden Actors`)
    (message `/Game/Blueprints/Interface/BI_HiddenHandler.Hide` _array_element)))

(event `self.Box.OnComponentBeginOverlap`
  (params (OverlappedComponent :type "PrimitiveComponent Object Reference") (OtherActor :type "Actor Object Reference") (OtherComp :type "PrimitiveComponent Object Reference") (OtherBodyIndex :type Integer) (bFromSweep :type Boolean) (SweepResult :type "HitResult Structure (by ref)"))
  (if (== OtherActor (`GameplayStatics.GetPlayerPawn` 0))
    (`/Engine/EditorBlueprintResources/StandardMacros.DoOnce` false
      (:`Completed`
        (`FXSystemComponent.SetColorParameter` (`self.Niagara`) "Color" (struct :`R` 0.0909 :`G` 1.0 :`B` 0.002387 :`A` 1.0))
        (`self.Hide/Unhide Actors`)
        (`KismetSystemLibrary.Delay` 2.0)
        (`self.K2_DestroyActor`)))))

(event `/Game/Blueprints/Interface/BI_HiddenHandler.Show Hidden`
  (`ActorComponent.Activate` (`self.Niagara`) true)
  (`self.SetActorHiddenInGame` false)
  (`self.SetActorEnableCollision` true))

(event `/Game/Blueprints/Interface/BI_HiddenHandler.Hide`
  (`ActorComponent.Deactivate` (`self.Niagara`))
  (`self.SetActorHiddenInGame` true)
  (`self.SetActorEnableCollision` false))

(fn `Get Tagged Actors and Save in Array`
  (`|ExecutionSequence`
    (:`then_0`
      (bind _outactors (`GameplayStatics.GetAllActorsWithTag` (`self.Hidden Actors Tag`)))
      (if (`KismetArrayLibrary.Array_IsNotEmpty` _outactors)
        (set `self.Hidden Actors` _outactors)
        (else
          (`KismetSystemLibrary.PrintString` "No Hidden Actors Tagged"))))
    (:`then_1`
      (bind _outactors_2 (`GameplayStatics.GetAllActorsWithTag` (`self.Actors To Hide Tag`)))
      (if (`KismetArrayLibrary.Array_IsNotEmpty` _outactors_2)
        (set `self.Actors To Hide` _outactors_2)
        (else
          (`KismetSystemLibrary.PrintString` "No Actors to Hide Tagged"))))))

(fn `Hide/Unhide Actors`
  (bind _hidden_actors (`self.Hidden Actors`))
  (bind _actors_to_hide (`self.Actors To Hide`))
  (`|ExecutionSequence`
    (:`then_0`
      (if (`KismetArrayLibrary.Array_IsNotEmpty` _hidden_actors)
        (`GameplayStatics.PlaySound2D` "/Game/Assets/Interface_And_Item_Sounds/Cues/Special_Powerup_03_Cue.Special_Powerup_03_Cue" 1.0 1.0 0.0 null null)
        (for _array_element _hidden_actors
          (message `/Game/Blueprints/Interface/BI_HiddenHandler.Show Hidden` _array_element))))
    (:`then_1`
      (if (`KismetArrayLibrary.Array_IsNotEmpty` _actors_to_hide)
        (for _array_element_2 _actors_to_hide
          (message `/Game/Blueprints/Interface/BI_HiddenHandler.Hide` _array_element_2))))))

(fn `UserConstructionScript`)