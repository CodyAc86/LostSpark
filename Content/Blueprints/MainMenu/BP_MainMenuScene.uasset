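; BP_MainMenuScene is the main menu scene actor that animates two Niagara effects from BeginPlay, where it also assigns a camera variable.
; Two timelines drive both effects' relative X and Z, with crossed tracks and a fixed Y on either side.
; The second timeline follows the first with swapped axis mapping, then reverses the first, whose completion restarts the second in an endless cycle.
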(event `self.ReceiveBeginPlay`
  (set `self.Camera` (`self.Camera`))
  (bind (_direction _z_mover _x_mover) (`Timeline|Timeline` :!label _label)
    (:`Update`
      (`SceneComponent.K2_SetRelativeTransform` (`self.Niagara2`) (`KismetMathLibrary.MakeTransform` (`KismetMathLibrary.MakeVector` _x_mover 174.580794 _z_mover)) false false)
      (`SceneComponent.K2_SetRelativeTransform` (`self.Niagara1`) (`KismetMathLibrary.MakeTransform` (`KismetMathLibrary.MakeVector` _z_mover -145.72204 _x_mover)) false false))
    (:`Finished`
      (bind (_direction_2 _z_mover_2 _x_mover_2) (`Timeline|Timeline_0` :!via `PlayFromStart`)
        (:`Update`
          (`SceneComponent.K2_SetRelativeTransform` (`self.Niagara2`) (`KismetMathLibrary.MakeTransform` (`KismetMathLibrary.MakeVector` _z_mover_2 174.580794 _x_mover_2)) false false)
          (`SceneComponent.K2_SetRelativeTransform` (`self.Niagara1`) (`KismetMathLibrary.MakeTransform` (`KismetMathLibrary.MakeVector` _x_mover_2 -145.72204 _z_mover_2)) false false))
        (:`Finished`
          (goto _label :!via `ReverseFromEnd`))))))

(fn `UserConstructionScript`)