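; Main menu game mode that determines which level the player last played.
; On BeginPlay it loads the LastPlayed save slot and caches its level name, defaulting to the tutorial level when no save exists.
; GetLastPlayedLevel exposes that name, while the score and UI stat functions are stubs returning zeros.
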(event `self.ReceiveBeginPlay`
  (bind _returnvalue (`GameplayStatics.DoesSaveGameExist` "LastPlayed"))
  (if _returnvalue
    (bind _returnvalue_2 (`GameplayStatics.LoadGameFromSlot` "LastPlayed"))
    (bind _output_get (set `self.Save Last Game Ref` _returnvalue_2))
    (bind _assave_last_played_level (cast `/Game/Saves/SaveLastPlayedLevel` _output_get))
    (set `self.Last Played Level Name` (`/Game/Saves/SaveLastPlayedLevel.LastPlayedLevel` _assave_last_played_level))
    (else
      (set `self.Last Played Level Name` "LVL1_Tutorial"))))

(fn `CalculateFinalScore`
  (returns (`Final Score` :type Integer) (`High Score` :type Integer) (`Collected Pickups` :type Integer) (`Max Collectibles` :type Integer) (`Completion Time` :type Integer))
  (return 0 0 0 0 0))

(fn `GetAllScores`
  (returns (`Final Score` :type Integer) (`High Score` :type Integer) (`Collected Pickups` :type Integer) (`Max Collectibles` :type Integer) (`Completion Time` :type "Float (double-precision)") (`Enemies Spawned` :type Integer) (`Enemies Defeated` :type Integer) (`Current Player Score` :type Integer) (`Minus Score Per Second` :type Integer) (`Level Completion Time Int` :type Integer) (`Minus Timer Score` :type Integer))
  (return 0 0 0 0 0.0 0 0 0 0 0 0))

(fn `GetLastPlayedLevel`
  (returns (LastPlayedLevel :type Name))
  (return (`self.Last Played Level Name`)))

(fn `GetScore`
  (returns (Score :type Integer))
  (return 0))

(fn `SendUIStats`
  (returns (HP :type "Float (double-precision)") (MaxHP :type "Float (double-precision)") (LVL :type Integer) (XP :type "Float (double-precision)") (LevelXP :type "Float (double-precision)") (`Boost Timer` :type "Float (double-precision)") (Sparks :type Integer))
  (return 0.0 0.0 0 0.0 0.0 0.0 0))

(fn `UserConstructionScript`)