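; BP_PowerCore is an interactable power core that switches a list of linked actors, apparently force fields, on and off.
; Player overlap toggles a highlight overlay and interactability; Interact plays sound and particles.
; It reads the last linked actor's status, swaps the emissive material and sends the opposite enable/disable message through BI_Interact.
; Separate routines force-disable linked actors, hide or show the core, and reveal hidden actors.
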(event `self.ReceiveBeginPlay`
  (bind _interactable_actors_list (`self.Interactable Actors List`))
  (if (`KismetArrayLibrary.Array_IsNotEmpty` _interactable_actors_list)
    (for _array_element _interactable_actors_list
      (bind _isactivated (message `/Game/Blueprints/Interface/BI_Interact.GetActiveStatus` _array_element)))
    (bind _output_get (set `self.AreActorsActivated` _isactivated))
    (if _output_get
      (`PrimitiveComponent.SetMaterialByName` (`self.SM_Desk_A_v3`) "EnergyEmissive_A" "/Game/StarterBundle/ModularScifiHallways/Materials/MI_EnergyEmissive_A.MI_EnergyEmissive_A")
      (else
        (`PrimitiveComponent.SetMaterialByName` (`self.SM_Desk_A_v3`) "EnergyEmissive_A" "/Game/StarterBundle/ModularScifiHallways/Materials/MI_EnergyEmissive_B.MI_EnergyEmissive_B")))
    (else
      (`KismetSystemLibrary.PrintString` "No force field Actors in array"))))

(event `self.Box Collision.OnComponentBeginOverlap`
  (params (OverlappedComponent :type "PrimitiveComponent Object Reference") (OtherActor :type "Actor Object Reference") (OtherComp :type "PrimitiveComponent Object Reference") (OtherBodyIndex :type Integer) (bFromSweep :type Boolean) (SweepResult :type "HitResult Structure (by ref)"))
  (`self.Has Interacted`
    (:`then`)
    (:`else`
      (if (== OtherActor (`GameplayStatics.GetPlayerCharacter` 0))
        (`self.Activate Highlight`)
        (set `self.CanInteract` true)))))

(event `self.Box Collision.OnComponentEndOverlap`
  (params (OverlappedComponent :type "PrimitiveComponent Object Reference") (OtherActor :type "Actor Object Reference") (OtherComp :type "PrimitiveComponent Object Reference") (OtherBodyIndex :type Integer))
  (if (== OtherActor (`GameplayStatics.GetPlayerCharacter` 0))
    (`self.Deactivate Highlight`)
    (set `self.CanInteract` false)))

(event `/Game/Blueprints/Interface/BI_Interact.Interact`
  (bind _interactable_actors_list (`self.Interactable Actors List`))
  (if (`self.Can Interact`)
    (`KismetSystemLibrary.PrintString` "Hello")
    (`GameplayStatics.PlaySound2D` "/Game/Assets/Interface_And_Item_Sounds/Cues/Futuristic_Click_04_Cue.Futuristic_Click_04_Cue" 1.0 1.0 0.0 null null)
    (`ActorComponent.Activate` (`self.NS_InteractParticles`) false)
    (if (`KismetArrayLibrary.Array_IsNotEmpty` _interactable_actors_list)
      (for _array_element _interactable_actors_list
        (bind _isactivated (message `/Game/Blueprints/Interface/BI_Interact.GetActiveStatus` _array_element)))
      (bind _output_get (set `self.AreActorsActivated` _isactivated))
      (if _output_get
        (`KismetSystemLibrary.PrintString` "Is Active")
        (`PrimitiveComponent.SetMaterialByName` (`self.SM_Desk_A_v3`) "EnergyEmissive_A" "/Game/StarterBundle/ModularScifiHallways/Materials/MI_EnergyEmissive_B.MI_EnergyEmissive_B")
        (for _array_element_2 (`self.Interactable Actors List`)
          (if (`KismetSystemLibrary.DoesImplementInterface` _array_element_2 "/Game/Blueprints/Interface/BI_Interact.BI_Interact_C")
            (message `/Game/Blueprints/Interface/BI_Interact.Disable` _array_element_2)
            (else
              (`KismetSystemLibrary.PrintString` "The actor in array does not implement interface BI_Interact"))))
        (else
          (`KismetSystemLibrary.PrintString` "is Disabled")
          (`PrimitiveComponent.SetMaterialByName` (`self.SM_Desk_A_v3`) "EnergyEmissive_A" "/Game/StarterBundle/ModularScifiHallways/Materials/MI_EnergyEmissive_A.MI_EnergyEmissive_A")
          (for _array_element_3 (`self.Interactable Actors List`)
            (if (`KismetSystemLibrary.DoesImplementInterface` _array_element_3 "/Game/Blueprints/Interface/BI_Interact.BI_Interact_C")
              (message `/Game/Blueprints/Interface/BI_Interact.Enable` _array_element_3)
              (else
                (`KismetSystemLibrary.PrintString` "The actor in array does not implement interface BI_Interact")))))))))

(event `Activate Highlight`
  (`MeshComponent.SetOverlayMaterial` (`self.SM_Desk_A_v3`) "/Game/Blueprints/Materials/MI_HighlightMat_Inst.MI_HighlightMat_Inst")
  (set `self.CanInteract` true))

(event `Deactivate Highlight`
  (`MeshComponent.SetOverlayMaterial` (`self.SM_Desk_A_v3`) null)
  (set `self.CanInteract` false))

(event `/Game/Blueprints/Interface/BI_Interact.Disable`
  (bind _interactable_actors_list (`self.Interactable Actors List`))
  (`ActorComponent.Activate` (`self.NS_InteractParticles`) false)
  (`PrimitiveComponent.SetMaterialByName` (`self.SM_Desk_A_v3`) "EnergyEmissive_A" "/Game/StarterBundle/ModularScifiHallways/Materials/MI_EnergyEmissive_B.MI_EnergyEmissive_B")
  (if (`KismetArrayLibrary.Array_IsNotEmpty` _interactable_actors_list)
    (for _array_element _interactable_actors_list
      (if (`KismetSystemLibrary.DoesImplementInterface` _array_element "/Game/Blueprints/Interface/BI_Interact.BI_Interact_C")
        (message `/Game/Blueprints/Interface/BI_Interact.Disable` _array_element)
        (else
          (`KismetSystemLibrary.PrintString` "The actor in array does not implement interface BI_Interact"))))))

(event `/Game/Blueprints/Interface/BI_HiddenHandler.Hide`
  (`self.SetActorHiddenInGame` true)
  (`self.SetActorEnableCollision` false))

(event `/Game/Blueprints/Interface/BI_HiddenHandler.Show Hidden`
  (`self.SetActorHiddenInGame` false)
  (`self.SetActorEnableCollision` true))

(fn `Activate Hidden Collectibles`
  (for _array_element (`self.Interactable Actors List`)
    (`self.SetActorHiddenInGame` _array_element false)
    (`self.SetActorEnableCollision` _array_element true)
    (set `self.Has Interacted` true)
    (`self.Deactivate Highlight`)))

(fn `Can Interact`
  (returns (ReturnValue :type Boolean))
  (`self.CanInteract`
    (:`then`
      (return (`KismetArrayLibrary.Array_IsNotEmpty` (`self.Interactable Actors List`))))
    (:`else`)))

(fn `GetActiveStatus`
  (returns (isActivated :type Boolean))
  (return false))

(fn `UserConstructionScript`)