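; Interactable desk-and-laptop console that highlights when the player enters its box and fires its effects on interaction.
; On BeginPlay it gathers tagged hidden actors, doors, power cores and target points, hiding the hidden actors.
; Interacting plays sound and particles, reveals those actors, opens doors, disables cores via interface, and spawns enemy sparks at target points.
; Each spawn raises the GameMode's max score, and the spawn count is reported afterward.
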(event `self.ReceiveBeginPlay`
  (bind _hidden_actors_list (`self.Hidden Actors List`))
  (bind _outactors (`GameplayStatics.GetAllActorsWithTag` (`self.Hidden Objects Tag`)))
  (set `self.Hidden Actors List` _outactors)
  (if (`KismetArrayLibrary.Array_IsNotEmpty` _hidden_actors_list)
    (for _array_element _hidden_actors_list
      (message `/Game/Blueprints/Interface/BI_HiddenHandler.Hide` _array_element)
      (bind _outactors_2 (`GameplayStatics.GetAllActorsWithTag` (`self.Door Tag`) :!label _label))
      (set `self.Interactable Doors` _outactors_2)
      (bind _outactors_3 (`GameplayStatics.GetAllActorsOfClassWithTag` "/Game/Blueprints/Interactables/BP_PowerCore.BP_PowerCore_C" (`self.Power Core Tag`)))
      (set `self.Power Cores` _outactors_3)
      (bind _outactors_4 (`GameplayStatics.GetAllActorsOfClassWithTag` "/Script/Engine.TargetPoint" (`self.Target Point Tag`)))
      (set `self.Target Points` _outactors_4))
    (else
      (goto _label))))

(event `self.Box Collision.OnComponentBeginOverlap`
  (params (OverlappedComponent :type "PrimitiveComponent Object Reference") (OtherActor :type "Actor Object Reference") (OtherComp :type "PrimitiveComponent Object Reference") (OtherBodyIndex :type Integer) (bFromSweep :type Boolean) (SweepResult :type "HitResult Structure (by ref)"))
  (`self.Has Interacted`
    (:`then`)
    (:`else`
      (if (== OtherActor (`GameplayStatics.GetPlayerCharacter` 0))
        (`self.Activate Highlight`)))))

(event `self.Box Collision.OnComponentEndOverlap`
  (params (OverlappedComponent :type "PrimitiveComponent Object Reference") (OtherActor :type "Actor Object Reference") (OtherComp :type "PrimitiveComponent Object Reference") (OtherBodyIndex :type Integer))
  (if (== OtherActor (`GameplayStatics.GetPlayerCharacter` 0))
    (`self.Deactivate Highlight`)))

(event `/Game/Blueprints/Interface/BI_Interact.Interact`
  (`self.CanInteract`
    (:`then`
      (`GameplayStatics.PlaySound2D` "/Game/SciFiUISFX/Cues/Glitches/Glitch_14_Cue.Glitch_14_Cue" 1.0 1.0 0.0 null null)
      (`ActorComponent.Activate` (`self.NS_InteractParticles`) false)
      (`|ExecutionSequence`
        (:`then_0`
          (`self.Activate Hidden Collectibles`))
        (:`then_1`
          (`self.Activate Door`))
        (:`then_2`
          (`self.Disable Power Cores`))
        (:`then_3`
          (`self.Spawn Enemy Sparks`))
        (:`then_4`
          (set `self.Has Interacted` true)
          (`self.Deactivate Highlight`))))
    (:`else`)))

(event `Activate Highlight`
  (`MeshComponent.SetOverlayMaterial` (`self.SM_Desk_A_v3`) "/Game/Blueprints/Materials/MI_HighlightMat_Inst.MI_HighlightMat_Inst")
  (`MeshComponent.SetOverlayMaterial` (`self.SM_Laptop`) "/Game/Blueprints/Materials/MI_HighlightMat_Inst.MI_HighlightMat_Inst")
  (set `self.CanInteract` true))

(event `Deactivate Highlight`
  (`MeshComponent.SetOverlayMaterial` (`self.SM_Desk_A_v3`) null)
  (`MeshComponent.SetOverlayMaterial` (`self.SM_Laptop`) null)
  (set `self.CanInteract` false))

(event `/Game/Blueprints/Interface/BI_HiddenHandler.Hide`
  (`self.SetActorHiddenInGame` true)
  (`self.SetActorEnableCollision` false))

(event `/Game/Blueprints/Interface/BI_HiddenHandler.Show Hidden`
  (`self.SetActorHiddenInGame` false)
  (`self.SetActorEnableCollision` true))

(fn `Activate Door`
  (bind _interactable_doors (`self.Interactable Doors`))
  (if (`KismetArrayLibrary.Array_IsNotEmpty` _interactable_doors)
    (for _array_element _interactable_doors
      (message `/Game/Blueprints/Interface/BI_Interact.Open` _array_element))
    (else
      (return))))

(fn `Activate Hidden Collectibles`
  (bind _hidden_actors_list (`self.Hidden Actors List`))
  (if (`KismetArrayLibrary.Array_IsNotEmpty` _hidden_actors_list)
    (`GameplayStatics.PlaySound2D` "/Game/Assets/Interface_And_Item_Sounds/Cues/Special_Powerup_03_Cue.Special_Powerup_03_Cue" 1.0 1.0 0.0 null null)
    (for _array_element _hidden_actors_list
      (message `/Game/Blueprints/Interface/BI_HiddenHandler.Show Hidden` _array_element)))
  (return))

(fn `Disable Power Cores`
  (bind _power_cores (`self.Power Cores`))
  (if (`KismetArrayLibrary.Array_IsNotEmpty` _power_cores)
    (for _array_element _power_cores
      (if (`KismetSystemLibrary.DoesImplementInterface` _array_element "/Game/Blueprints/Interface/BI_Interact.BI_Interact_C")
        (`/Game/Blueprints/Interface/BI_Interact.Disable` _array_element)
        (else
          (`KismetSystemLibrary.PrintString` "No Power Core with implemented interface")
          (return)))))
  (return))

(fn `GetActiveStatus`
  (returns (isActivated :type Boolean))
  (return false))

(fn `Is Door Actors Array Empty`
  (returns (ReturnValue :type Boolean))
  (return (`KismetArrayLibrary.Array_IsEmpty` (`self.Interactable Doors`))))

(fn `Is Hidden Actors Array Empty`
  (returns (ReturnValue :type Boolean))
  (return (`KismetArrayLibrary.Array_IsEmpty` (`self.Hidden Actors List`))))

(fn `Spawn Enemy Sparks`
  (bind _returnvalue (`GameplayStatics.GetGameMode`))
  (if (`KismetArrayLibrary.Array_IsNotEmpty` (`self.Target Points`))
    (for _array_element (`self.Target Points`)
      (`|SpawnActorFromClass` "/Game/Blueprints/Enemy_AI/BP_EnemySpark.BP_EnemySpark_C" (`self.GetTransform` _array_element) "Undefined" "MultiplyWithRoot" null 8.0 null)
      (`/Engine/EditorBlueprintResources/StandardMacros.IncrementInt` (`self.Spawned Enemies Count`)
        (:`  `
          (message `/Game/Variant_SideScroller/Blueprints/BPI_SideScrolling.UpdateCurrentLevelMaxScore` _returnvalue (`self.Score Per Spawned Enemy`)))))
    (message `/Game/Variant_SideScroller/Blueprints/BPI_SideScrolling.UpdateEnemiesSpawnedCount` _returnvalue (`self.Spawned Enemies Count`)))
  (return))

(fn `UserConstructionScript`)