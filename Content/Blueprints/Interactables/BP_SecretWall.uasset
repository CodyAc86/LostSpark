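; BP_SecretWall is an interactable hidden wall that opens when Interact is called, then removes itself.
; Open plays a mechanical lock sound, then the RotateWall timeline sets the actor's rotation.
; When that finishes, the Mover timeline slides it along world X by subtracting from its current location each update, then destroys the actor.
; GetActiveStatus always returns false.
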(event `self.ReceiveBeginPlay`)

(event `/Game/Blueprints/Interface/BI_Interact.Open`
  (`GameplayStatics.PlaySound2D` "/Game/Assets/Audio/Latches_Mechanical_Lock_Unlock_SFX__270__Cue.Latches_Mechanical_Lock_Unlock_SFX__270__Cue" 1.0 1.0 0.0 null null)
  (bind (_direction _rotateup) (`Timeline|RotateWall`)
    (:`Update`
      (`self.K2_SetActorRotation` (`KismetMathLibrary.MakeRotator` 0.0 _rotateup)))
    (:`Finished`
      (bind (_direction_2 _x_axis_location) (`Timeline|Mover`)
        (:`Update`
          (bind (_returnvalue_x _returnvalue_y _returnvalue_z) (`self.Get Current Location`))
          (`self.K2_SetActorLocation` (`KismetMathLibrary.MakeVector` (- _returnvalue_x _x_axis_location) _returnvalue_y _returnvalue_z)))
        (:`Finished`
          (`self.K2_DestroyActor`))))))

(event `/Game/Blueprints/Interface/BI_Interact.Interact`
  (`/Game/Blueprints/Interface/BI_Interact.Open`))

(fn `Get Current Location`
  (returns (ReturnValue_X :type "Float (double-precision)") (ReturnValue_Y :type "Float (double-precision)") (ReturnValue_Z :type "Float (double-precision)"))
  (bind (_returnvalue_x _returnvalue_y _returnvalue_z) (`KismetMathLibrary.BreakVector` (`self.K2_GetActorLocation`)))
  (return _returnvalue_x _returnvalue_y _returnvalue_z))

(fn `GetActiveStatus`
  (returns (isActivated :type Boolean))
  (return false))

(fn `UserConstructionScript`)