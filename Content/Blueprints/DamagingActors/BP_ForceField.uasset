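; Electric force field hazard that stuns and damages actors entering its box, and can be enabled, disabled, hidden or shown.
; Box overlaps fill an actor list, sending freeze messages through BI_StopAllMovement and starting a fast looping, never-cleared timer that damages listed actors still inside.
; End overlap removes actors and tells the player to stop damage when outside.
; Activation toggles Niagara effects, sound and overlap events together, tracked by IsActivated.
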(event `self.ReceiveBeginPlay`
  (`self.isActivated`
    (:`then`
      (`/Game/Blueprints/Interface/BI_Interact.Enable`))
    (:`else`
      (`/Game/Blueprints/Interface/BI_Interact.Disable`))))

(event `self.Box.OnComponentBeginOverlap`
  (params (OverlappedComponent :type "PrimitiveComponent Object Reference") (OtherActor :type "Actor Object Reference") (OtherComp :type "PrimitiveComponent Object Reference") (OtherBodyIndex :type Integer) (bFromSweep :type Boolean) (SweepResult :type "HitResult Structure (by ref)"))
  (`/Engine/EditorBlueprintResources/StandardMacros.IsValid` OtherActor
    (:`Is Valid`
      (`KismetArrayLibrary.Array_AddUnique` (`self.Overlapping Actors`) OtherActor)
      (for _array_element (`self.Overlapping Actors`)
        (if (`KismetSystemLibrary.DoesImplementInterface` _array_element "/Game/Blueprints/Interface/BI_StopAllMovement.BI_StopAllMovement_C")
          (message `/Game/Blueprints/Interface/BI_StopAllMovement.Freeze` _array_element (`self.Stun Duration`))
          (`KismetSystemLibrary.K2_SetTimerDelegate` (delegate `Damage Actor`) 0.05 true))))))

(event `Damage Actor`
  (for _array_element (`self.Overlapping Actors`)
    (if (`PrimitiveComponent.IsOverlappingActor` (`self.Box`) _array_element)
      (`self.Damage Overlapping Actor`))))

(event `self.Box.OnComponentEndOverlap`
  (params (OverlappedComponent :type "PrimitiveComponent Object Reference") (OtherActor :type "Actor Object Reference") (OtherComp :type "PrimitiveComponent Object Reference") (OtherBodyIndex :type Integer))
  (bind _returnvalue (`GameplayStatics.GetPlayerCharacter` 0))
  (bind _returnvalue_2 (`KismetArrayLibrary.Array_RemoveItem` (`self.Overlapping Actors`) OtherActor))
  (if _returnvalue_2
    (if (not (`PrimitiveComponent.IsOverlappingActor` (`self.Box`) _returnvalue))
      (message `/Game/Blueprints/Interface/BI_StopDamage.Stop Damage` _returnvalue))))

(event `/Game/Blueprints/Interface/BI_Interact.Disable`
  (`self.Deactivate Force Field`))

(event `/Game/Blueprints/Interface/BI_Interact.Enable`
  (`self.Activate Force Field`))

(event `/Game/Blueprints/Interface/BI_HiddenHandler.Hide`
  (`self.SetActorHiddenInGame` true)
  (`self.SetActorEnableCollision` false))

(event `/Game/Blueprints/Interface/BI_HiddenHandler.Show Hidden`
  (`self.SetActorHiddenInGame` false)
  (`self.SetActorEnableCollision` true))

(fn `Activate Force Field`
  (bind _sc_electricforcefield (`self.SC_ElectricForcefield`))
  (`ActorComponent.Activate` (`self.NS_Electrified3`) false)
  (`ActorComponent.Activate` (`self.NS_Electrified2`) false)
  (`ActorComponent.Activate` (`self.Niagara1`) false)
  (`ActorComponent.Activate` (`self.NS_Electrified1`) false)
  (`ActorComponent.Activate` (`self.NS_Electrified`) false)
  (`ActorComponent.Activate` (`self.Niagara`) false)
  (`ActorComponent.Activate` (`self.Niagara2`) false)
  (if (not (`AudioComponent.IsPlaying` _sc_electricforcefield))
    (`AudioComponent.Play` _sc_electricforcefield 0.0))
  (set `PrimitiveComponent.bGenerateOverlapEvents` true (`self.Box`))
  (set `self.isActivated` true))

(fn `Damage Overlapping Actor`
  (for _array_element (`self.Overlapping Actors`)
    (if (`PrimitiveComponent.IsOverlappingActor` (`self.Box`) _array_element)
      (`GameplayStatics.ApplyDamage` _array_element (`self.Base Damage`)))))

(fn `Deactivate Force Field`
  (`ActorComponent.Deactivate` (`self.NS_Electrified3`))
  (`ActorComponent.Deactivate` (`self.NS_Electrified2`))
  (`ActorComponent.Deactivate` (`self.Niagara1`))
  (`ActorComponent.Deactivate` (`self.NS_Electrified1`))
  (`ActorComponent.Deactivate` (`self.NS_Electrified`))
  (`ActorComponent.Deactivate` (`self.Niagara`))
  (`ActorComponent.Deactivate` (`self.Niagara2`))
  (`AudioComponent.Stop` (`self.SC_ElectricForcefield`))
  (set `PrimitiveComponent.bGenerateOverlapEvents` false (`self.Box`))
  (set `self.isActivated` false))

(fn `GetActiveStatus`
  (returns (isActivated :type Boolean))
  (return (`self.isActivated`)))

(fn `UserConstructionScript`)