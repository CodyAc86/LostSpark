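; BP_DamageFloor is a hazard actor that continuously damages an actor standing inside its Box trigger.
; Box overlap stores a single DamagedActor and starts a very fast looping timer that applies BaseDamage while the overlap holds.
; End overlap clears the stored actor, first calling StopDamageMessage if it is the player character.
; The timer is never cleared, and its handler repeats that player cleanup whenever the overlap check fails.
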(event `self.Box.OnComponentBeginOverlap`
  (params (OverlappedComponent :type "PrimitiveComponent Object Reference") (OtherActor :type "Actor Object Reference") (OtherComp :type "PrimitiveComponent Object Reference") (OtherBodyIndex :type Integer) (bFromSweep :type Boolean) (SweepResult :type "HitResult Structure (by ref)"))
  (`/Engine/EditorBlueprintResources/StandardMacros.IsValid` OtherActor
    (:`Is Valid`
      (set `self.Damaged Actor` OtherActor)
      (`KismetSystemLibrary.K2_SetTimerDelegate` (delegate `StartDamaging`) 0.005 true))))

(event `StartDamaging`
  (bind _returnvalue (`GameplayStatics.GetPlayerCharacter` 0))
  (if (`PrimitiveComponent.IsOverlappingActor` (`self.Box`) (`self.Damaged Actor`))
    (`GameplayStatics.ApplyDamage` (`self.Damaged Actor`) (`self.Base Damage`) null self)
    (elif (== (`self.Damaged Actor`) _returnvalue)
      (message `/Game/Blueprints/Interface/BI_StopDamage.Stop Damage` _returnvalue)
      (set `self.Damaged Actor` null))))

(event `self.Box.OnComponentEndOverlap`
  (params (OverlappedComponent :type "PrimitiveComponent Object Reference") (OtherActor :type "Actor Object Reference") (OtherComp :type "PrimitiveComponent Object Reference") (OtherBodyIndex :type Integer))
  (if (== (`self.Damaged Actor`) (`GameplayStatics.GetPlayerCharacter` 0))
    (message `/Game/Blueprints/Interface/BI_StopDamage.Stop Damage` (`GameplayStatics.GetPlayerCharacter` 0))
    (set `self.Damaged Actor` null)
    (else
      (set `self.Damaged Actor` null))))

(fn `UserConstructionScript`)